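; BP_Generator drives level progression for a maze game, creating and persisting each level across three difficulty modes.
; The construction script builds the mode/level table of maze sizes, NPC spawns and dynamic-wall flags.
; Begin resets or restores progress; NextLevel advances and saves it.
; Generate runs Start only for unsaved levels, saves the layout under a mode+level slot, then always spawns BP_Game to load that slot.
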(event `self.ReceiveBeginPlay`)

(event `Begin`
  (params (newGame :type Boolean))
  (`|ExecutionSequence`
    (:`then_0`
      (bind _returnvalue (`GameplayStatics.CreateSaveGameObject` "/Game/Skripsi/Blueprints/BP_SaveGameLevelMode.BP_SaveGameLevelMode_C"))
      (set `self.saveGameLevelMode` _returnvalue)
      (if newGame
        (`self.DeleteAllSave`)
        (set `self.indexMode` 0 :!label _label)
        (set `self.indexLevel` 0)
        (set `self.slotName` (`KismetStringLibrary.Concat_StrStr` (`KismetStringLibrary.Conv_IntToString` (`self.indexMode`)) (`KismetStringLibrary.Conv_IntToString` (`self.indexLevel`))))
        (else
          (bind _returnvalue_2 (`GameplayStatics.DoesSaveGameExist` (`self.slotNameLevelMode`)))
          (if _returnvalue_2
            (bind _returnvalue_3 (`GameplayStatics.LoadGameFromSlot` (`self.slotNameLevelMode`)))
            (bind _asbp_save_game_level_mode (cast `/Game/Skripsi/Blueprints/BP_SaveGameLevelMode` _returnvalue_3))
            (bind _output_get (set `self.saveGameLevelMode` _asbp_save_game_level_mode))
            (set `self.indexMode` (`/Game/Skripsi/Blueprints/BP_SaveGameLevelMode.mode` _output_get))
            (set `self.indexLevel` (`/Game/Skripsi/Blueprints/BP_SaveGameLevelMode.level` _output_get))
            (set `self.slotName` (`KismetStringLibrary.Concat_StrStr` (`KismetStringLibrary.Conv_IntToString` (`self.indexMode`)) (`KismetStringLibrary.Conv_IntToString` (`self.indexLevel`))))
            (else
              (goto _label))))))
    (:`then_1`
      (bind _returnvalue_4 (`GameplayStatics.CreateSaveGameObject` "/Game/Skripsi/Blueprints/BP_SaveGame.BP_SaveGame_C"))
      (set `self.saveGame` _returnvalue_4)
      (`self.Generate`))))

(event `Generate`
  (bind (_mazesize _spawnnpcattacker _spawnnpcdisturber _generatedynamicwallandswitch) (break `/Game/Skripsi/Blueprints/S_Level` (`|GetArrayItem` (`.levels_3_809AF8C749EA2F1858EA58947F988FD8` (break `/Game/Skripsi/Blueprints/S_Mode` (`|GetArrayItem` (`self.mode`) (`self.indexMode`)))) (`self.indexLevel`))))
  (bind _returnvalue (`GameplayStatics.DoesSaveGameExist` (`self.slotName`)))
  (if _returnvalue
    (bind _returnvalue_2 (`|SpawnActorFromClass` "/Game/Skripsi/Blueprints/BP_Game.BP_Game_C" (`KismetMathLibrary.MakeTransform` (0.0 0.0 0.0)) "AlwaysSpawn" "OverrideRootScale" null self null))
    (`/Game/Skripsi/Blueprints/BP_Game.LoadGame_Event` _returnvalue_2 (`self.slotName`) (`self.indexMode`) (`self.indexLevel`))
    (else
      (`self.Start` _mazesize false 0.4 3 _spawnnpcattacker _spawnnpcdisturber _generatedynamicwallandswitch)
      (`self.SaveGames` (`self.slotName`))
      (bind _returnvalue_3 (`|SpawnActorFromClass` "/Game/Skripsi/Blueprints/BP_Game.BP_Game_C" (`KismetMathLibrary.MakeTransform` (0.0 0.0 0.0)) "AlwaysSpawn" "OverrideRootScale" null self null))
      (`/Game/Skripsi/Blueprints/BP_Game.LoadGame_Event` _returnvalue_3 (`self.slotName`) (`self.indexMode`) (`self.indexLevel`)))))

(event `NextLevel`
  (bind _savegamelevelmode (`self.saveGameLevelMode`))
  (bind _savegamelevelmode_2 (`self.saveGameLevelMode`))
  (`|ExecutionSequence`
    (:`then_0`
      (if (== (`self.indexLevel`) (`KismetArrayLibrary.Array_LastIndex` (`.levels_3_809AF8C749EA2F1858EA58947F988FD8` (break `/Game/Skripsi/Blueprints/S_Mode` (`|GetArrayItem` (`self.mode`) (`self.indexMode`))))))
        (if (not (== (`self.indexMode`) (`KismetArrayLibrary.Array_LastIndex` (`self.mode`))))
          (`/Engine/EditorBlueprintResources/StandardMacros.IncrementInt` (`self.indexMode`)
            (:`  `
              (set `self.indexLevel` 0)
              (set `self.slotName` (`KismetStringLibrary.Concat_StrStr` (`KismetStringLibrary.Conv_IntToString` (`self.indexMode`)) (`KismetStringLibrary.Conv_IntToString` (`self.indexLevel`))))
              (set `/Game/Skripsi/Blueprints/BP_SaveGameLevelMode.mode` (`self.indexMode`) _savegamelevelmode_2)
              (set `/Game/Skripsi/Blueprints/BP_SaveGameLevelMode.level` (`self.indexLevel`) _savegamelevelmode_2)
              (`GameplayStatics.SaveGameToSlot` (`self.saveGameLevelMode`) (`self.slotNameLevelMode`)))))
        (else
          (`/Engine/EditorBlueprintResources/StandardMacros.IncrementInt` (`self.indexLevel`)
            (:`  `
              (set `self.slotName` (`KismetStringLibrary.Concat_StrStr` (`KismetStringLibrary.Conv_IntToString` (`self.indexMode`)) (`KismetStringLibrary.Conv_IntToString` (`self.indexLevel`))))
              (set `/Game/Skripsi/Blueprints/BP_SaveGameLevelMode.mode` (`self.indexMode`) _savegamelevelmode)
              (set `/Game/Skripsi/Blueprints/BP_SaveGameLevelMode.level` (`self.indexLevel`) _savegamelevelmode)
              (`GameplayStatics.SaveGameToSlot` (`self.saveGameLevelMode`) (`self.slotNameLevelMode`)))))))
    (:`then_1`
      (`self.Generate`))))

(fn `DeleteAllSave`
  (locals (slot :type String))
  (bind _slotnamelevelmode (`self.slotNameLevelMode`))
  (bind _slot (`local.slot`))
  (`|ExecutionSequence`
    (:`then_0`
      (bind _returnvalue (`GameplayStatics.DoesSaveGameExist` _slotnamelevelmode))
      (if _returnvalue
        (`GameplayStatics.DeleteGameInSlot` _slotnamelevelmode)))
    (:`then_1`
      (for (_array_element _array_index) (`self.mode`)
        (for (_ _array_index_2) (`.levels_3_809AF8C749EA2F1858EA58947F988FD8` (break `/Game/Skripsi/Blueprints/S_Mode` _array_element))
          (set `local.slot` (`KismetStringLibrary.Concat_StrStr` (`KismetStringLibrary.Conv_IntToString` _array_index) (`KismetStringLibrary.Conv_IntToString` _array_index_2)))
          (bind _returnvalue_2 (`GameplayStatics.DoesSaveGameExist` _slot))
          (if _returnvalue_2
            (`GameplayStatics.DeleteGameInSlot` _slot)))))))

(fn `SaveGames`
  (params (slotName :type String))
  (locals (L_wall :type "Array of /Game/Skripsi/Blueprints/S_ArrayBool Structure") (L_NPC :type "Array of NPC Structure"))
  (`|ExecutionSequence`
    (:`then_0`
      ;[1 1 1] wall maze
      (for _array_element (`self.cells`)
        (`KismetArrayLibrary.Array_Add` (`local.L_wall`) (make `/Game/Skripsi/Blueprints/S_ArrayBool` (`.wall` (break `Cell` _array_element))))))
    (:`then_1`
      ;[1 1 1] npc
      (`|ExecutionSequence`
        (:`then_0`
          (for _array_element_2 (`self.NPCAttackers`)
            (`KismetArrayLibrary.Array_Add` (`local.L_NPC`) _array_element_2)))
        (:`then_1`
          (for _array_element_3 (`self.NPCDisturbers`)
            (`KismetArrayLibrary.Array_Add` (`local.L_NPC`) _array_element_3)))))
    (:`then_2`
      ;[1 1 1] Comment
      (set `/Game/Skripsi/Blueprints/BP_SaveGame.saveGame` (make `/Game/Skripsi/Blueprints/S_SaveGame` (`self.mazeSize`) (`self.gridSize`) (`local.L_wall`) (`local.L_NPC`) (`self.switch_`) (`self.dynamicWall`) (`self.paths`) (`self.NPCCollisionDatas`) (`self.playerSpawnLoc`) (`self.finishLoc`)) (`self.saveGame`))
      (bind _returnvalue (`GameplayStatics.SaveGameToSlot` (`self.saveGame`) slotName))
      (if _returnvalue
        (`KismetSystemLibrary.PrintString` (`KismetStringLibrary.Concat_StrStr` "SAVE SLOT " slotName) false)))))

(fn `SetModeLevel`
  (set `self.mode` (`|MakeArray` (make `/Game/Skripsi/Blueprints/S_Mode` (`|MakeArray` (make `/Game/Skripsi/Blueprints/S_Level` (make `IntPoint` 5 5) (make `SpawnNPCAttacker` true) (make `SpawnNPCDisturber` true)) (make `/Game/Skripsi/Blueprints/S_Level` (make `IntPoint` 5 5) (make `SpawnNPCAttacker` true) (make `SpawnNPCDisturber` true) true))) (make `/Game/Skripsi/Blueprints/S_Mode` (`|MakeArray` (make `/Game/Skripsi/Blueprints/S_Level` (make `IntPoint` 6 6) (make `SpawnNPCAttacker` false 0 1) (make `SpawnNPCDisturber` true)) (make `/Game/Skripsi/Blueprints/S_Level` (make `IntPoint` 7 7) (make `SpawnNPCAttacker` false 0 1) (make `SpawnNPCDisturber` true) true) (make `/Game/Skripsi/Blueprints/S_Level` (make `IntPoint` 8 8) (make `SpawnNPCAttacker` false 0 1) (make `SpawnNPCDisturber` false 0 1) true) (make `/Game/Skripsi/Blueprints/S_Level` (make `IntPoint` 9 9) (make `SpawnNPCAttacker` false 0 2) (make `SpawnNPCDisturber` false 0 1) true) (make `/Game/Skripsi/Blueprints/S_Level` (make `IntPoint` 10 10) (make `SpawnNPCAttacker` false 0 2) (make `SpawnNPCDisturber` false 0 1) true))) (make `/Game/Skripsi/Blueprints/S_Mode` (`|MakeArray` (make `/Game/Skripsi/Blueprints/S_Level` (make `IntPoint` 10 10) (make `SpawnNPCAttacker` false 0 1 1) (make `SpawnNPCDisturber` false 0 1) true) (make `/Game/Skripsi/Blueprints/S_Level` (make `IntPoint` 10 10) (make `SpawnNPCAttacker` false 0 1 1) (make `SpawnNPCDisturber` false 0 0 1) true) (make `/Game/Skripsi/Blueprints/S_Level` (make `IntPoint` 10 10) (make `SpawnNPCAttacker` true 2) (make `SpawnNPCDisturber` true 2) true))))))

(fn `UserConstructionScript`
  (`self.SetModeLevel`))